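; Treasure chest actor that prompts the nearby player, opens to award score and can end the game.
; Box overlap shows or removes one of two widgets created at BeginPlay, chosen by whether the first-person character's score exceeds a threshold.
; NewFunction, not called within this Blueprint, runs once to animate both chest meshes and add points.
; Reaching the score target then shows a delayed game-over screen, pauses and enables the cursor.
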(event OnComponentBeginOverlap(Box)
  (params (OverlappedComponent :type Primitive%20Component%20Object%20Reference) (OtherActor :type Actor%20Object%20Reference) (OtherComp :type Primitive%20Component%20Object%20Reference) (OtherBodyIndex :type Integer) (bFromSweep :type Boolean) (SweepResult :type Hit%20Result%20Structure%20%28by%20ref%29))
  (bind _returnvalue (Game|GetPlayerCharacter 0))
  ;[1 1 1] instruction
  (if (== OtherActor _returnvalue)
    (bind _asbp_first_person_character (Utilities|Casting|CastToBP_FirstPersonCharacter _returnvalue))
    (if (> (Variables|/Game/FirstPerson/Blueprints/BP_FirstPersonCharacter.BP_FirstPersonCharacter_C|Getscore _asbp_first_person_character) 20)
      (UserInterface|Viewport|AddtoViewport (Variables|Default|Getchestwidget1) 0)
      (else
        (UserInterface|Viewport|AddtoViewport (Variables|Default|Getchestwidget2) 0)))))

(event OnComponentEndOverlap(Box)
  (params (OverlappedComponent :type Primitive%20Component%20Object%20Reference) (OtherActor :type Actor%20Object%20Reference) (OtherComp :type Primitive%20Component%20Object%20Reference) (OtherBodyIndex :type Integer))
  (bind _returnvalue (Game|GetPlayerCharacter 0))
  ;[1 1 1] instruction
  (if (== OtherActor _returnvalue)
    (bind _asbp_first_person_character (Utilities|Casting|CastToBP_FirstPersonCharacter _returnvalue))
    (if (> (Variables|/Game/FirstPerson/Blueprints/BP_FirstPersonCharacter.BP_FirstPersonCharacter_C|Getscore _asbp_first_person_character) 20)
      (Widget|RemovefromParent (Variables|Default|Getchestwidget1))
      (else
        (Widget|RemovefromParent (Variables|Default|Getchestwidget2))))))

(event EventBeginPlay
  ;[1 1 1] instruction
  (bind _returnvalue (UserInterface|CreateWidget "/Game/PICKUP/Chest_Widget.Chest_Widget_C"))
  (Variables|Default|Setchestwidget1 _returnvalue)
  (bind _returnvalue_2 (UserInterface|CreateWidget "/Game/PICKUP/Chest_Widget2.Chest_Widget2_C"))
  (Variables|Default|Setchestwidget2 _returnvalue_2))

(event Collision|EventActorBeginOverlap
  (params (OtherActor :type Actor%20Object%20Reference)))

(event EventTick
  (params (DeltaSeconds :type Float%20%28single-precision%29)))

(event EventNewFunction
  (bind _returnvalue (Game|GetPlayerController 0))
  (Utilities|FlowControl|DoOnce false
    (:Completed
      (Components|Animation|PlayAnimation (Variables|Default|GetSkeletalMesh) "/Game/PICKUP/bot_Anim.bot_Anim" false)
      (Components|Animation|PlayAnimation (Variables|Default|GetSkeletalMesh1) "/Game/PICKUP/top_Anim.top_Anim" false)
      (bind _asbp_first_person_character (Utilities|Casting|CastToBP_FirstPersonCharacter (Game|GetPlayerCharacter 0)))
      (Variables|/Game/FirstPerson/Blueprints/BP_FirstPersonCharacter.BP_FirstPersonCharacter_C|Setscore _asbp_first_person_character (+ (Variables|/Game/FirstPerson/Blueprints/BP_FirstPersonCharacter.BP_FirstPersonCharacter_C|Getscore _asbp_first_person_character) 100))
      (if (not (< (Variables|/Game/FirstPerson/Blueprints/BP_FirstPersonCharacter.BP_FirstPersonCharacter_C|Getscore _asbp_first_person_character) 200))
        (Utilities|FlowControl|Delay 1.0)
        (bind _returnvalue_2 (UserInterface|CreateWidget "/Game/FirstPerson/UI/WBP_GameOver.WBP_GameOver_C"))
        (UserInterface|Viewport|AddtoViewport _returnvalue_2 0)
        (Game|SetGamePaused true)
        (Input|SetInputModeGameandUI _returnvalue 0 "DoNotLock" true false)
        (Variables|/Script/Engine.PlayerController|SetbShowMouseCursor _returnvalue true)))))

(fn ConstructionScript)